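; Interactable door that the player opens and closes, with a lockable state, sounds and Russian action prompts.
; MakeAction routes to DoorMove, which plays or reverses a rotation timeline, choosing swing direction from the player's side of the door.
; When locked, a closed door plays a rattle timeline and sound, while an open one can still close.
; The construction script poses initially open doors in either direction.
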(event Custom|DoorLockedMove
  (Utilities|FlowControl|DoOnce false :!label _label
    (:Completed
      (if (Variables|Default|Getclosed)
        (Utilities|FlowControl|DoOnce false :!label _label_2
          (:Completed
            (Audio|PlaySound2D "/Game/Lexi4/Door/DoorSounds/DoorLocked.DoorLocked" 5.0 1.0 0.0 0 0)
            (bind _lockeddoor (Timeline|DoorLockedRotate PlayFromStart)
              (:Update
                (Transformation|SetRelativeRotation (Variables|Default|GetDoor) (Math|Rotator|MakeRotator 0.0 0.0 _lockeddoor) false false))
              (:Finished
                (goto _label_2 Reset)))))
        (else
          (Utilities|FlowControl|Sequence
            (:then_0
              (Utilities|FlowControl|DoOnce false :!label _label_3
                (:Completed
                  (if (Variables|Default|Getclosed)
                    (Audio|PlaySound2D "/Game/Lexi4/Door/DoorSounds/DoorOpen.DoorOpen" 1.0 1.0 0.0 0 0)
                    (Utilities|GetOpenDirection)
                    (Variables|Default|Setclosed false)
                    (bind _newtrack_0 (Timeline|DoorOpenRotate Play)
                      (:Update
                        (Utilities|FlowControl|Gate true
                          (:Exit
                            (Transformation|SetRelativeRotation (Variables|Default|GetDoor) (Math|Rotator|MakeRotator 0.0 0.0 (* (Variables|Default|GetDirection) _newtrack_0)) false false))))
                      (:Finished
                        (goto _label_3 Reset)))
                    (else
                      (Audio|PlaySound2D "/Game/Lexi4/Door/DoorSounds/DoorClose.DoorClose" 1.0 1.0 0.0 0 0)
                      (Variables|Default|Setclosed true)
                      (Timeline|DoorOpenRotate Reverse))))))
            (:then_1
              (Utilities|FlowControl|Delay 1.0)
              (goto _label Reset))))))))

(event Custom|DoorMove
  (Utilities|FlowControl|DoOnce false :!label _label
    (:Completed
      (if (Variables|Default|Getclosed)
        (Audio|PlaySound2D "/Game/Lexi4/Door/DoorSounds/DoorOpen.DoorOpen" 1.0 1.0 0.0 0 0)
        (Utilities|GetOpenDirection)
        (Variables|Default|Setclosed false)
        (bind _newtrack_0 (Timeline|DoorOpenRotate Play)
          (:Update
            (Utilities|FlowControl|Gate true
              (:Exit
                (Transformation|SetRelativeRotation (Variables|Default|GetDoor) (Math|Rotator|MakeRotator 0.0 0.0 (* (Variables|Default|GetDirection) _newtrack_0)) false false))))
          (:Finished
            (goto _label Reset)))
        (else
          (Audio|PlaySound2D "/Game/Lexi4/Door/DoorSounds/DoorClose.DoorClose" 1.0 1.0 0.0 0 0)
          (Variables|Default|Setclosed true)
          (Timeline|DoorOpenRotate Reverse))))))

(event Custom|SetMoveOpened
  (bind _newtrack_0 (Timeline|DoorOpenRotate SetNewTime)
    (:Update
      (Utilities|FlowControl|Gate true
        (:Exit
          (Transformation|SetRelativeRotation (Variables|Default|GetDoor) (Math|Rotator|MakeRotator 0.0 0.0 (* (Variables|Default|GetDirection) _newtrack_0)) false false))))
    (:Finished
      (Utilities|FlowControl|DoOnce false) ; enters at Reset
    )))

(event EventBeginPlay
  (Utilities|FlowControl|Gate true) ; enters at Open
)

(event EventLockUnlockDoor
  (params (Lock :type Boolean))
  (Variables|Default|SetLocked Lock))

(fn ConstructionScript
  (bind _initopendirection (Variables|Default|GetInitOpenDirection))
  (if (not (Variables|Default|Getclosed))
    (CallFunction|SetMoveOpened)
    (Transformation|SetRelativeRotation (Variables|Default|GetDoor) (select _initopendirection "0,90.000000, 0" "0,-90.000000, 0") false false)
    (Variables|Default|SetDirection (select _initopendirection 1.0 -1.0))))

(fn CanInteract
  (return true))

(fn GetActionText
  (return (select (and (Variables|Default|GetLocked) (Variables|Default|Getclosed)) "Ты ключ дома забыл?" (select (Variables|Default|Getclosed) "Открыть дверь" "Закрыть дверь"))))

(fn MakeAction
  (if (Variables|Default|GetLocked)
    (CallFunction|DoorLockedMove)
    (else
      (CallFunction|DoorMove)
      (return true))))