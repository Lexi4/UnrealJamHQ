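; Interactable electrical panel that opens on first use and switches off the electricity on the next.
; Two DoOnce gates stage this: opening plays an animation, changes the prompt to "turn off electricity" (in Russian) and unlocks the switch step.
; Switching plays a turn animation, messages every OVR_LightSwitch_Interface actor, disables further interaction and enables the Printer.
; Small functions expose the prompt, interact state, enabling and action.
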(event Custom|Interact
  (bind _skeletalmesh (Variables|Default|GetSkeletalMesh))
  (Utilities|FlowControl|Sequence
    (:then_0
      (Utilities|FlowControl|DoOnce true :!label _label
        (:Completed
          (Components|Animation|PlayAnimation _skeletalmesh "/Game/Lexi4/OVR/Animations/OVR_Anim_Turn.OVR_Anim_Turn" false)
          (Utilities|FlowControl|Delay 0.2)
          (bind _outactors (Actor|GetAllActorswithInterface "/Game/Lexi4/OVR/OVR_LightSwitch_Interface.OVR_LightSwitch_Interface_C"))
          (for _array_element _outactors
            (Class|OVRLightSwitchInterface|TurnLight(Message) _array_element)
            (Variables|Default|SetCanInteract? false)
            (Default|Enable (Variables|Default|GetPrinter))))))
    (:then_1
      (Utilities|FlowControl|DoOnce false
        (:Completed
          (Components|Animation|PlayAnimation _skeletalmesh "/Game/Lexi4/OVR/Animations/OVR_Anim_Armature_Armature_Otkr_Otkr.OVR_Anim_Armature_Armature_Otkr_Otkr" false)
          (Utilities|FlowControl|Delay 2.6)
          (Variables|Default|SetInterText "Выключить электричество")
          (goto _label Reset))))))

(fn ConstructionScript)

(fn LockUnlockDoor
  (return false false))

(fn CanInteract
  (return (Variables|Default|GetCanInteract?)))

(fn Enable
  (Variables|Default|SetCanInteract? true)
  (return true))

(fn GetActionText
  (return (Variables|Default|GetInterText)))

(fn MakeAction
  (CallFunction|Interact)
  (return true))