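; BP_Ammo_Box_01 is an interactable ammo pickup for rifles, pistols or shotguns.
; Its construction script turns a Melee or None weapon type into Rifle.
; It is always interactable and shows a Russian pickup prompt matching its weapon type.
; On action, it casts player pawn 0 to BP_Unreal_Jam_Player_01, adds its ammo count for that type and destroys itself, reporting whether the cast succeeded.
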(event EventBeginPlay)

(event Collision|EventActorBeginOverlap
  (params (OtherActor :type Actor%20Object%20Reference)))

(event EventTick
  (params (DeltaSeconds :type Float%20%28single-precision%29)))

(fn ConstructionScript
  (if (or (Utilities|Enum|Equal(Enum) (Variables|Settings|GetWeaponType) "NewEnumerator3") (Utilities|Enum|Equal(Enum) (Variables|Settings|GetWeaponType) "NewEnumerator4"))
    (Variables|Settings|SetWeaponType "NewEnumerator0")))

(fn CanInteract
  (return true))

(fn GetActionText
  (return (Utilities|Select :Index (Variables|Settings|GetWeaponType) :NewEnumerator0 "Подобрать патроны для автомата" :NewEnumerator1 "Подобрать патроны для пистолета" :NewEnumerator2 "Подобрать патроны для дробовика" :NewEnumerator3 "" :NewEnumerator4 "")))

(fn MakeAction
  (bind _asbp_unreal_jam_player_01 (Utilities|Casting|CastToBP_Unreal_Jam_Player_01 (Game|Player|GetPlayerPawn 0))
    (:then
      (Default|AddAmmo _asbp_unreal_jam_player_01 (Variables|Settings|GetAmmoCount) (Variables|Settings|GetWeaponType))
      (Actor|DestroyActor self)
      (return true))
    (:CastFailed
      (return false))))