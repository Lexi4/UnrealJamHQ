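; BP_Exit_Office_01 is an interactable exit from the office that takes the player to the Parking level.
; It allows interaction only when no actors tagged Enemy remain, and shows a Russian action prompt to go out to the parking lot.
; On use it saves the player through the game instance and plays a sound.
; It also has the player controller fade out, then opens the level after a short delay.
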(event Custom|StartTravel
  (bind _asbp_unreal_jam_player_controller_01 (Utilities|Casting|CastToBP_Unreal_Jam_Player_Controller_01 (Game|GetPlayerController 0)))
  (Default|FadeOut _asbp_unreal_jam_player_controller_01)
  (Utilities|FlowControl|Delay 2.0)
  (Game|OpenLevel(byName) "Parking"))

(event EventBeginPlay)

(event Collision|EventActorBeginOverlap
  (params (OtherActor :type Actor%20Object%20Reference)))

(event EventTick
  (params (DeltaSeconds :type Float%20%28single-precision%29)))

(fn ConstructionScript)

(fn CanInteract
  (bind _outactors (Actor|GetAllActorswithTag "Enemy"))
  (return (<= (Utilities|Array|Length _outactors) 0)))

(fn GetActionText
  (return "Выйти на парковку"))

(fn MakeAction
  (Default|SavePlayer (CallFunction|GetUJGameInstance))
  (CallFunction|StartTravel)
  (Audio|PlaySound2D "/Game/Dialogues/Scenario/A_14_Ez_Brz_01.A_14_Ez_Brz_01" 1.0 1.0 0.0 0 0)
  (return true))