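; Base first aid kit pickup that the player can use to restore health through an interaction.
; CanInteract and MakeAction look up the health system component on player 0's pawn and check CanUseAid.
; A successful use passes RestoreHealth to AddRestoreHealth and destroys the kit.
; GetActionText supplies a Russian "Use first aid kit" prompt; the event graph and construction script are empty.
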(event EventBeginPlay)

(event Collision|EventActorBeginOverlap
  (params (OtherActor :type Actor%20Object%20Reference)))

(event EventTick
  (params (DeltaSeconds :type Float%20%28single-precision%29)))

(fn ConstructionScript)

(fn CanInteract
  (bind _asbp_unreal_jam_player_01 (Utilities|Casting|CastToBP_Unreal_Jam_Player_01 (Game|Player|GetPlayerPawn 0))
    (:then
      (Utilities|IsValid (Actor|GetComponentbyClass _asbp_unreal_jam_player_01 "/Game/Lucas/BP_Unreal_Jam_Health_System_01.BP_Unreal_Jam_Health_System_01_C")
        (:Is%20Valid
          (return (Default|CanUseAid (Actor|GetComponentbyClass _asbp_unreal_jam_player_01 "/Game/Lucas/BP_Unreal_Jam_Health_System_01.BP_Unreal_Jam_Health_System_01_C"))))
        (:Is%20Not%20Valid
          (return false))))
    (:CastFailed
      (return false))))

(fn GetActionText
  (return "Использовать аптечку"))

(fn MakeAction
  (bind _asbp_unreal_jam_player_01 (Utilities|Casting|CastToBP_Unreal_Jam_Player_01 (Game|Player|GetPlayerPawn 0))
    (:then
      (Utilities|IsValid (Actor|GetComponentbyClass _asbp_unreal_jam_player_01 "/Game/Lucas/BP_Unreal_Jam_Health_System_01.BP_Unreal_Jam_Health_System_01_C")
        (:Is%20Valid
          (if (Default|CanUseAid (Actor|GetComponentbyClass _asbp_unreal_jam_player_01 "/Game/Lucas/BP_Unreal_Jam_Health_System_01.BP_Unreal_Jam_Health_System_01_C"))
            (Default|AddRestoreHealth (Actor|GetComponentbyClass _asbp_unreal_jam_player_01 "/Game/Lucas/BP_Unreal_Jam_Health_System_01.BP_Unreal_Jam_Health_System_01_C") (Variables|Settings|GetRestoreHealth))
            (Actor|DestroyActor self)
            (return true)
            (else
              (return false))))
        (:Is%20Not%20Valid
          (return false))))
    (:CastFailed
      (return false))))