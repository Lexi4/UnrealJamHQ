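; BP_Locker_01 is a searchable locker that gives the player a weapon.
; It exposes interaction functions: an availability check, a re-enable function, a Russian "Search" prompt and the action itself.
; Searching clears its CanInteract flag, then adds a fixed weapon enum to the player pawn's owned weapons, switches to it and plays a 2D sound.
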(event EventBeginPlay)

(event Collision|EventActorBeginOverlap
  (params (OtherActor :type Actor%20Object%20Reference)))

(event EventTick
  (params (DeltaSeconds :type Float%20%28single-precision%29)))

(fn ConstructionScript)

(fn CanInteract
  (return (Variables|Default|GetbCanInteract)))

(fn Enable
  (Variables|Default|SetbCanInteract true)
  (return false))

(fn GetActionText
  (return "Обыскать"))

(fn MakeAction
  (Variables|Default|SetbCanInteract false)
  (bind _asbp_unreal_jam_player_01 (Utilities|Casting|CastToBP_Unreal_Jam_Player_01 (Game|Player|GetPlayerPawn 0))
    (:then
      (Utilities|Array|Add (Variables|/Game/Lucas/BP_Unreal_Jam_Player_01.BP_Unreal_Jam_Player_01_C|GetOwnedWeapons _asbp_unreal_jam_player_01) "NewEnumerator2")
      (Default|SwitchWeapon _asbp_unreal_jam_player_01 "NewEnumerator2")
      (Audio|PlaySound2D "/Game/Dialogues/Scenario/A_11_Now_We_Talking_01.A_11_Now_We_Talking_01" 1.0 1.0 0.0 0 0)
      (return true))
    (:CastFailed
      (return false))))