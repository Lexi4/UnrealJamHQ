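; Trigger-driven actor that plays an assigned sound when its TriggerFired event runs.
; It calls the parent trigger logic, then branches on IsUISound to play the sound either in 2D or at a world location.
; The positional sound plays from the Sphere component's center, offset along its up vector by half the sphere radius.
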(event EventBeginPlay
  (|CallParentFunction) ; This node is disabled and will not be called.\nDrag off pins to build functionality.
)

(event Collision|EventActorBeginOverlap
  (params (OtherActor :type Actor%20Object%20Reference))
  (|CallParentFunction OtherActor) ; This node is disabled and will not be called.\nDrag off pins to build functionality.
)

(event EventTick
  (params (DeltaSeconds :type Float%20%28single-precision%29))
  (|CallParentFunction DeltaSeconds) ; This node is disabled and will not be called.\nDrag off pins to build functionality.
)

(event EventTriggerFired
  (bind _sphere (Variables|Default|GetSphere))
  (|CallParentFunction)
  (if (Variables|Default|GetbIsUISound)
    (Audio|PlaySound2D (Variables|Default|GetSoundToPlay) 1.0 1.0 0.0 0 0)
    (else
      (Audio|PlaySoundatLocation (Variables|Default|GetSoundToPlay) (+ (Transformation|GetWorldLocation _sphere) (* (Math|Vector|GetUpVector _sphere) (* (Variables|/Script/Engine.SphereComponent|GetSphereRadius _sphere) 0.5))) "0, 0, 0" 1.0 1.0 0.0 0 0 0))))

(fn ConstructionScript
  (|CallParentFunction))