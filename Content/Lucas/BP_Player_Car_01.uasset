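; Player car interactable offering a "drive home" action, whose first use with no tagged enemies on the map triggers an ambush.
; DeployEnemies disables input, turns the camera to the car's spotlight via timeline, honks, lights up, spawns enemies at relative offsets, then rotates back and restores input.
; Later uses play a one-time warning while enemies remain, or the drive-home voice line once cleared, then disable interaction.
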(event Custom|DeployEnemies
  (bind _returnvalue (Game|GetPlayerController 0))
  (bind _returnvalue_2 (Game|GetPlayerController 0))
  (bind _returnvalue_3 (Pawn|GetControlRotation _returnvalue_2 :!class /Script/Engine.Controller))
  (Input|DisableInput (Game|Player|GetPlayerPawn 0) _returnvalue_2)
  (Variables|Default|SetStartRotation _returnvalue_3)
  (Variables|Default|SetTargetRotation (Math|Rotator|MakeRotator 0.0 (.Pitch (Math|Rotator|BreakRotator _returnvalue_3)) (.yaw (Math|Rotator|FindLookatRotation (Transformation|GetWorldLocation (Variables|/Script/Engine.Actor|GetRootComponent (Game|Player|GetPlayerPawn 0))) (Transformation|GetWorldLocation (Variables|Default|GetSpotLight1))))))
  (bind _time (Timeline|Timeline_0 PlayFromStart)
    (:Update
      (Pawn|SetControlRotation (Game|GetPlayerController 0) (Math|Rotator|MakeRotator 0.0 (.pitch (Math|Rotator|CombineRotators (Variables|Default|GetStartRotation) (* (Math|Rotator|Delta(Rotator) (Variables|Default|GetTargetRotation) (Variables|Default|GetStartRotation)) _time))) (.yaw (Math|Rotator|CombineRotators (Variables|Default|GetStartRotation) (* (Math|Rotator|Delta(Rotator) (Variables|Default|GetTargetRotation) (Variables|Default|GetStartRotation)) _time))))))
    (:Finished
      (Audio|PlaySound2D "/Game/Sounds/A_Car_Horn_01.A_Car_Horn_01" 1.0 1.0 0.0 0 0)
      (Rendering|Components|Light|SetIntensity (Variables|Default|GetSpotLight) 1e+04)
      (Rendering|Components|Light|SetIntensity (Variables|Default|GetSpotLight1) 1e+04)
      (Variables|Default|SetbCanInteract false)
      (Utilities|FlowControl|Delay 1.5)
      (for _array_element (Variables|Default|GetEnemiesPositions)
        (bind _returnvalue_4 (Game|SpawnActorfromClass "/Game/Lucas/BP_Unreal_Jam_Enemy_Base_01.BP_Unreal_Jam_Enemy_Base_01_C" (Math|Transform|MakeTransform (+ (Math|Vector|MakeVector (.x _array_element) (.z _array_element) 5e+01) (Transformation|GetActorLocation)) "0,180.000000, 0" "1,1,1") "AlwaysSpawn" 0 0))
        (Default|StartAI _returnvalue_4))
      (Variables|Default|SetbCanInteract true)
      (Input|DisableInput (Game|Player|GetPlayerPawn 0) _returnvalue)
      (Variables|Default|SetStartRotation (Pawn|GetControlRotation _returnvalue :!class /Script/Engine.Controller))
      (Variables|Default|SetTargetRotation (Math|Rotator|MakeRotator 0.0 0.0 0.0))
      (bind _time_2 (Timeline|Timeline_1 PlayFromStart)
        (:Update
          (Pawn|SetControlRotation (Game|GetPlayerController 0) (Math|Rotator|MakeRotator 0.0 (.pitch (Math|Rotator|CombineRotators (Variables|Default|GetStartRotation) (* (Math|Rotator|Delta(Rotator) (Variables|Default|GetTargetRotation) (Variables|Default|GetStartRotation)) _time_2))) (.yaw (Math|Rotator|CombineRotators (Variables|Default|GetStartRotation) (* (Math|Rotator|Delta(Rotator) (Variables|Default|GetTargetRotation) (Variables|Default|GetStartRotation)) _time_2))))))
        (:Finished
          (Input|EnableInput (Game|Player|GetPlayerPawn 0) (Game|GetPlayerController 0)))))))

(event EventBeginPlay)

(event Collision|EventActorBeginOverlap
  (params (OtherActor :type Actor%20Object%20Reference)))

(event EventTick
  (params (DeltaSeconds :type Float%20%28single-precision%29)))

(fn ConstructionScript)

(fn IsEnemiesonMap
  (bind _outactors (Actor|GetAllActorswithTag "Enemy"))
  (return (> (Utilities|Array|Length _outactors) 0)))

(fn CanInteract
  (return (and (Variables|Default|GetbCanInteract) (or (not (Variables|Default|GetbWasWarningSpoken)) (not (CallFunction|IsEnemiesonMap))))))

(fn GetActionText
  (return "Уехать домой"))

(fn MakeAction
  (if (Variables|Default|GetbFirst)
    (if (CallFunction|IsEnemiesonMap)
      (return true)
      (else
        (CallFunction|DeployEnemies)
        (Variables|Default|SetbFirst false)
        (return true)))
    (elif (CallFunction|IsEnemiesonMap)
      (if (not (Variables|Default|GetbWasWarningSpoken))
        (Variables|Default|SetbWasWarningSpoken true)
        (Audio|PlaySound2D "/Game/Dialogues/Scenario/A_19_Need_To_Kill_Remain_01.A_19_Need_To_Kill_Remain_01" 1.0 1.0 0.0 0 0)
        (return true))
      (else
        (Variables|Default|SetbCanInteract false)
        (Audio|PlaySound2D "/Game/Dialogues/Scenario/A_22_Nothing_Happens_On_Way_Home_01.A_22_Nothing_Happens_On_Way_Home_01" 1.0 1.0 0.0 0 0)
        (return true)))))