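; BP_Police_Car_01 is a searchable police car that gives the player a weapon, apparently a rifle judging by its sound cue.
; Interaction functions show a Russian "Search" prompt and allow the action only until WasFound is set.
; MakeAction casts player pawn 0 to the jam player, sets WasFound, adds and equips the weapon, and plays a 2D found-rifle sound.
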(event EventBeginPlay)

(event Collision|EventActorBeginOverlap
  (params (OtherActor :type Actor%20Object%20Reference)))

(event EventTick
  (params (DeltaSeconds :type Float%20%28single-precision%29)))

(fn ConstructionScript)

(fn CanInteract
  (return (not (Variables|Default|GetbWasFound))))

(fn GetActionText
  (return "Обыскать"))

(fn MakeAction
  (bind _asbp_unreal_jam_player_01 (Utilities|Casting|CastToBP_Unreal_Jam_Player_01 (Game|Player|GetPlayerPawn 0))
    (:then
      (Variables|Default|SetbWasFound true)
      (Utilities|Array|Add (Variables|/Game/Lucas/BP_Unreal_Jam_Player_01.BP_Unreal_Jam_Player_01_C|GetOwnedWeapons _asbp_unreal_jam_player_01) "NewEnumerator0")
      (Default|SwitchWeapon _asbp_unreal_jam_player_01 "NewEnumerator0")
      (Audio|PlaySound2D "/Game/Dialogues/Scenario/A_21_Found_Rifle_01.A_21_Found_Rifle_01" 1.0 1.0 0.0 0 0)
      (return true))
    (:CastFailed
      (return false))))