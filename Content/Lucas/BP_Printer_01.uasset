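; Interactable office printer that the player can knock away, showing a Russian prompt about hating cartridge refills.
; Enable works in two stages: the first call sets it alive, the next makes it killable, which CanInteract requires until it is dead.
; MakeAction plays a sound, messages ActorToEnable, calls Dead and launches the physics-enabled CoffeBoiler component horizontally away from the player, aimed through the Fire component.
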(event EventBeginPlay)

(event Collision|EventActorBeginOverlap
  (params (OtherActor :type Actor%20Object%20Reference)))

(event EventTick
  (params (DeltaSeconds :type Float%20%28single-precision%29)))

(fn ConstructionScript)

(fn GetActionText
  (return "Я ненавижу заправлять картриджи!"))

(fn CanInteract
  (return (Math|Boolean|ANDBoolean (Variables|Default|GetbIsAlive) (not (Variables|Default|GetbIsDead)) (Variables|Default|GetbCanBeKilled))))

(fn MakeAction
  (bind _returnvalue (Game|GetPlayerCharacter 0))
  (bind _fire (Variables|Default|GetFire))
  (bind _returnvalue_2 (Transformation|GetWorldLocation _fire))
  (bind _capsulecomponent (Variables|/Script/Engine.Character|GetCapsuleComponent _returnvalue))
  (bind _returnvalue_3 (Transformation|GetWorldLocation _capsulecomponent))
  (bind _returnvalue_4 (Math|Vector|GetUpVector _capsulecomponent))
  (bind _capsulehalfheight (Variables|/Script/Engine.CapsuleComponent|GetCapsuleHalfHeight _capsulecomponent))
  (bind _returnvalue_5 (* _returnvalue_4 _capsulehalfheight))
  (bind _returnvalue_6 (* _returnvalue_5 1.5))
  (bind _returnvalue_7 (+ _returnvalue_3 _returnvalue_6))
  (bind _returnvalue_8 (- _returnvalue_2 _returnvalue_7))
  (if (Variables|Default|GetbIsAlive)
    (Audio|PlaySound2D "/Game/Dialogues/Scenario/A_07_Whoops_01.A_07_Whoops_01" 1.0 1.0 0.0 0 0)
    (Class|BPEnableInterface01|Enable(Message) (Variables|Default|GetActorToEnable))
    (Variables|Default|SetbIsDead true)
    (CallFunction|Dead)
    (Physics|SetSimulatePhysics (Variables|Default|GetCoffeBoiler) true)
    (Physics|AddImpulse (Variables|Default|GetCoffeBoiler) (* (Math|Vector|Normalize (Math|Vector|MakeVector (.x _returnvalue_8) (.y _returnvalue_8) 0.0)) 1e+03) "None" true)
    (return false)))

(fn Enable
  (if (Variables|Default|GetbIsAlive)
    (Variables|Default|SetbCanBeKilled true)
    (else
      (Variables|Default|SetbIsAlive true)))
  (return true))