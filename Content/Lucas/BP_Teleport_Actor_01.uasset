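; Trigger-driven teleport actor that moves the player pawn to a new position behind a screen fade.
; When its inherited TriggerFired event runs, it disables player input and has the custom player controller fade out.
; After a delay, it places the pawn at TeleportLocation offset from the actor's own location and applies TeleportRotation as control rotation.
; It then fades back in and restores input after a shorter delay.
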(event EventBeginPlay)

(event Collision|EventActorBeginOverlap
  (params (OtherActor :type Actor%20Object%20Reference)))

(event EventTick
  (params (DeltaSeconds :type Float%20%28single-precision%29)))

(event EventTriggerFired
  (|CallParentFunction)
  (Input|DisableInput (Game|Player|GetPlayerPawn 0) (Game|GetPlayerController 0))
  (bind _asbp_unreal_jam_player_controller_01 (Utilities|Casting|CastToBP_Unreal_Jam_Player_Controller_01 (Game|GetPlayerController 0)))
  (Default|FadeOut _asbp_unreal_jam_player_controller_01)
  (Utilities|FlowControl|Delay 2.0)
  (Transformation|SetActorLocation (Game|Player|GetPlayerPawn 0) (+ (Variables|Default|GetTeleportLocation) (Transformation|GetActorLocation)) false false)
  (Pawn|SetControlRotation (Game|GetPlayerController 0) (Variables|Default|GetTeleportRotation))
  (bind _asbp_unreal_jam_player_controller_01_2 (Utilities|Casting|CastToBP_Unreal_Jam_Player_Controller_01 (Game|GetPlayerController 0)))
  (Default|Fadein _asbp_unreal_jam_player_controller_01_2)
  (Utilities|FlowControl|Delay 1.0)
  (Input|EnableInput (Game|Player|GetPlayerPawn 0) (Game|GetPlayerController 0)))

(fn ConstructionScript
  (|CallParentFunction))