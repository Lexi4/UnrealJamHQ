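; Test actor that acts as a constant damage beam along its Arrow component's forward direction.
; Each Tick it runs a complex line trace on a fixed channel from the arrow, drawing the ray for debugging.
; Hit actors implementing BP_Unreal_Jam_Damage_Interface_01 receive a fixed damage message every frame, so total damage scales with frame rate.
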(event EventBeginPlay)

(event Collision|EventActorBeginOverlap
  (params (OtherActor :type Actor%20Object%20Reference)))

(event EventTick
  (params (DeltaSeconds :type Float%20%28single-precision%29))
  (bind _arrow (Variables|Default|GetArrow))
  (bind _returnvalue (Transformation|GetWorldLocation _arrow))
  (bind (_outhit _returnvalue_2) (Collision|LineTraceByChannel _returnvalue (+ _returnvalue (* (Math|Vector|GetForwardVector _arrow) 1e+03)) "TraceTypeQuery4" true 0 "ForDuration" true "(R=1.000000,G=0.000000,B=0.000000,A=1.000000)" "(R=0.000000,G=1.000000,B=0.000000,A=1.000000)" DeltaSeconds))
  (if _returnvalue_2
    (if (Utilities|DoesObjectImplementInterface (.HitActor (Collision|BreakHitResult _outhit)) "/Game/Lucas/BP_Unreal_Jam_Damage_Interface_01.BP_Unreal_Jam_Damage_Interface_01_C")
      (Class|BPUnrealJamDamageInterface01|ReceiveDamage(Message) (.HitActor (Collision|BreakHitResult _outhit)) 1e+01))))

(fn ConstructionScript)