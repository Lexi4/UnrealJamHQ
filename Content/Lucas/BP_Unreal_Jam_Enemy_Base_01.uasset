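; Base melee enemy that chases the player with looping AI MoveTo at a randomized walk speed once StartAI is called.
; Tick triggers a repeating attack montage within attack range and applies damage once per StartHit/EndHit window when the capsule overlaps the player.
; ReceiveDamage handles death: ragdoll, stopped movement, cleared tags, kill sound, OnDead notification and timed removal.
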(event OnComponentBeginOverlap(Capsule)
  (params (OverlappedComponent :type Primitive%20Component%20Object%20Reference) (OtherActor :type Actor%20Object%20Reference) (OtherComp :type Primitive%20Component%20Object%20Reference) (OtherBodyIndex :type Integer) (bFromSweep :type Boolean) (SweepResult :type Hit%20Result%20Structure%20%28by%20ref%29)))

(event Custom|HuntCharacter
  (if (> (Variables|Settings|GetHealth) 0.0)
    (AI|AIMoveTo self "0, 0, 0" (Game|Player|GetPlayerPawn 0) 0.0 false
      (:OnSuccess
        (CallFunction|HuntCharacter)))))

(event Custom|StartAI
  (CallFunction|HuntCharacter))

(event Custom|Hit
  (if (> (Variables|Settings|GetHealth) 0.0)
    (Animation|Montage|PlayMontage (Variables|Character|GetMesh) (Variables|Settings|GetAttackMontage)
      (:OnCompleted
        (if (Variables|Default|GetbIsAttack)
          (CallFunction|Hit))))))

(event EventBeginPlay
  (Variables|/Script/Engine.CharacterMovementComponent|SetMaxWalkSpeed (Variables|Character|GetCharacterMovement) (Math|Random|RandomFloatinRange 425.0 275.0)))

(event Collision|EventActorBeginOverlap
  (params (OtherActor :type Actor%20Object%20Reference)))

(event EventTick
  (params (DeltaSeconds :type Float%20%28single-precision%29))
  (Utilities|IsValid (Game|Player|GetPlayerPawn 0)
    (:Is%20Valid
      (if (Variables|Default|GetbIsAttack)
        (if (and (Variables|Default|GetbCanDamage) (not (Variables|Default|GetbOverlappedCurrentHit)))
          (if (Collision|IsOverlappingActor (Variables|Default|GetCapsule) (Game|Player|GetPlayerPawn 0) :!class /Script/Engine.PrimitiveComponent)
            (Variables|Default|SetbOverlappedCurrentHit true)
            (Class|BPUnrealJamDamageInterface01|ReceiveDamage(Message) (Game|Player|GetPlayerPawn 0) (Variables|Default|GetDamage))))
        (elif (<= (Transformation|GetDistanceTo (Game|Player|GetPlayerPawn 0) self) (Variables|Settings|GetStartAttackDistance))
          (Variables|Default|SetbIsAttack true)
          (CallFunction|Hit))))))

(fn ConstructionScript)

(fn Activate)

(fn StartHit
  (Variables|Default|SetbCanDamage true)
  (Variables|Default|SetbOverlappedCurrentHit false))

(fn EndHit
  (Variables|Default|SetbCanDamage false))

(fn ReceiveDamage
  (params (Damage :type Float%20%28single-precision%29))
  (if (> (Variables|Settings|GetHealth) 0.0)
    (bind _output_get (Variables|Settings|SetHealth (- (Variables|Settings|GetHealth) Damage)))
    (if (<= _output_get 0.0)
      (Variables|/Script/Engine.SkeletalMeshComponent|SetbPauseAnims (Variables|Character|GetMesh) true)
      (Physics|SetSimulatePhysics (Variables|Character|GetMesh) true)
      (Collision|SetCollisionEnabled (Variables|Collision|GetCapsuleComponent) "NoCollision")
      (Actor|SetLifeSpan self 3e+01)
      (AI|Navigation|StopMovement (Pawn|GetController))
      (CallFunction|EndHit)
      (Utilities|Array|Clear (Variables|Actor|GetTags))
      (Default|PlayKillSound (CallFunction|GetUJGameInstance))
      (Default|CallOnDead)
      (return true)
      (else
        (return true)))))