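; Game instance for the Unreal Jam shooter that carries player state and provides shared UI and audio helpers.
; SavePlayer and LoadPlayer copy ammo, weapons and health between the player pawn and instance variables, re-equipping through SwitchWeapon.
; It creates the ammo widget and a cached interaction prompt.
; PlayMusic endlessly alternates two fading ambient tracks that persist across levels, while voice functions play random pickup, kill and hurt barks by weighted chance.
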(event Custom|MakeAmmoWidget
  (bind _returnvalue (UserInterface|CreateWidget "/Game/Lucas/W_Unreal_Jam_Ammo_Widget_01.W_Unreal_Jam_Ammo_Widget_01_C" (Game|GetPlayerController 0)))
  (Variables|Default|SetAmmoWidget _returnvalue)
  (UserInterface|Viewport|AddtoViewport (Variables|Default|GetAmmoWidget) 100))

(event Custom|PlayMusic
  (bind _returnvalue (Audio|SpawnSound2D (Utilities|Array|Get(acopy) (Utilities|Array|MakeArray "/Game/Music/A_Ambient_01.A_Ambient_01" "/Game/Music/A_Ambient_02.A_Ambient_02") (Math|Integer|SelectInt 0 1 (Variables|Default|GetbMusicFlag))) 0.65 1.0 0.0 0 true))
  (Audio|Components|Audio|FadeIn _returnvalue 2.0 1.0 0.0 :!class /Script/Engine.AudioComponent)
  (Utilities|FlowControl|Delay (- (Variables|/Script/Engine.SoundBase|GetDuration (Variables|/Script/Engine.AudioComponent|GetSound _returnvalue)) 2.0))
  (Audio|Components|Audio|FadeOut _returnvalue 2.0 0.0 :!class /Script/Engine.AudioComponent)
  (Variables|Default|SetbMusicFlag (not (Variables|Default|GetbMusicFlag)))
  (CallFunction|PlayMusic))

(fn EnabledActionStroke
  (params (ActionText :type Text))
  (Utilities|IsValid (Variables|Default|GetActionStroke)
    (:Is%20Valid
      (if (UserInterface|Viewport|IsinViewport (Variables|Default|GetActionStroke))
        _
        (else
          (UserInterface|Viewport|AddtoViewport (Variables|Default|GetActionStroke) 15 :!label _label))))
    (:Is%20Not%20Valid
      (bind _returnvalue (UserInterface|CreateWidget "/Game/Lucas/W_Unreal_Jam_Interaction_Stroke_01.W_Unreal_Jam_Interaction_Stroke_01_C" (Game|GetPlayerController 0)))
      (Variables|Default|SetActionStroke _returnvalue)
      (goto _label)))
  (Default|SetActionText (Variables|Default|GetActionStroke) ActionText)
  (Default|ToggleVisibility (Variables|Default|GetActionStroke) true))

(fn DisableActionStroke
  (Utilities|IsValid (Variables|Default|GetActionStroke)
    (:Is%20Valid
      _)
    (:Is%20Not%20Valid
      (bind _returnvalue (UserInterface|CreateWidget "/Game/Lucas/W_Unreal_Jam_Interaction_Stroke_01.W_Unreal_Jam_Interaction_Stroke_01_C" (Game|GetPlayerController 0)))
      (Variables|Default|SetActionStroke _returnvalue)))
  (Default|ToggleVisibility (Variables|Default|GetActionStroke) false))

(fn SavePlayer
  (bind _asbp_unreal_jam_player_01 (Utilities|Casting|CastToBP_Unreal_Jam_Player_01 (Game|Player|GetPlayerPawn 0)))
  (Variables|Default|SetRifleMagAmmo (Variables|/Game/Lucas/BP_Unreal_Jam_Player_01.BP_Unreal_Jam_Player_01_C|GetRifleMagAmmo _asbp_unreal_jam_player_01))
  (Variables|Default|SetRifleTotalAmmo (Variables|/Game/Lucas/BP_Unreal_Jam_Player_01.BP_Unreal_Jam_Player_01_C|GetRifleTotalAmmo _asbp_unreal_jam_player_01))
  (Variables|Default|SetPistolMagAmmo (Variables|/Game/Lucas/BP_Unreal_Jam_Player_01.BP_Unreal_Jam_Player_01_C|GetPistolMagAmmo _asbp_unreal_jam_player_01))
  (Variables|Default|SetPistolTotalAmmo (Variables|/Game/Lucas/BP_Unreal_Jam_Player_01.BP_Unreal_Jam_Player_01_C|GetPistolTotalAmmo _asbp_unreal_jam_player_01))
  (Variables|Default|SetShotgunMagAmmo (Variables|/Game/Lucas/BP_Unreal_Jam_Player_01.BP_Unreal_Jam_Player_01_C|GetShotgunMagAmmo _asbp_unreal_jam_player_01))
  (Variables|Default|SetShotgunTotalAmmo (Variables|/Game/Lucas/BP_Unreal_Jam_Player_01.BP_Unreal_Jam_Player_01_C|GetShotgunTotalAmmo _asbp_unreal_jam_player_01))
  (Variables|Default|SetCurrentWeapon (Variables|/Game/Lucas/BP_Unreal_Jam_Player_01.BP_Unreal_Jam_Player_01_C|GetCurrentWeapon _asbp_unreal_jam_player_01))
  (Variables|Default|SetOwnedWeapons (Variables|/Game/Lucas/BP_Unreal_Jam_Player_01.BP_Unreal_Jam_Player_01_C|GetOwnedWeapons _asbp_unreal_jam_player_01))
  (Variables|Default|SetHealth (Variables|/Game/Lucas/BP_Unreal_Jam_Health_System_01.BP_Unreal_Jam_Health_System_01_C|GetHealth (Variables|/Game/Lucas/BP_Unreal_Jam_Player_01.BP_Unreal_Jam_Player_01_C|GetBP_Unreal_Jam_Health_System_01 _asbp_unreal_jam_player_01)))
  (Variables|Default|SetRemainHelth (Variables|/Game/Lucas/BP_Unreal_Jam_Health_System_01.BP_Unreal_Jam_Health_System_01_C|GetRemainRestoreHealth (Variables|/Game/Lucas/BP_Unreal_Jam_Player_01.BP_Unreal_Jam_Player_01_C|GetBP_Unreal_Jam_Health_System_01 _asbp_unreal_jam_player_01))))

(fn LoadPlayer
  (bind _asbp_unreal_jam_player_01 (Utilities|Casting|CastToBP_Unreal_Jam_Player_01 (Game|Player|GetPlayerPawn 0)))
  (Variables|/Game/Lucas/BP_Unreal_Jam_Player_01.BP_Unreal_Jam_Player_01_C|SetRifleMagAmmo _asbp_unreal_jam_player_01 (Variables|Default|GetRifleMagAmmo))
  (Variables|/Game/Lucas/BP_Unreal_Jam_Player_01.BP_Unreal_Jam_Player_01_C|SetRifleTotalAmmo _asbp_unreal_jam_player_01 (Variables|Default|GetRifleTotalAmmo))
  (Variables|/Game/Lucas/BP_Unreal_Jam_Player_01.BP_Unreal_Jam_Player_01_C|SetPistolMagAmmo _asbp_unreal_jam_player_01 (Variables|Default|GetPistolMagAmmo))
  (Variables|/Game/Lucas/BP_Unreal_Jam_Player_01.BP_Unreal_Jam_Player_01_C|SetPistolTotalAmmo _asbp_unreal_jam_player_01 (Variables|Default|GetPistolTotalAmmo))
  (Variables|/Game/Lucas/BP_Unreal_Jam_Player_01.BP_Unreal_Jam_Player_01_C|SetShotgunMagAmmo _asbp_unreal_jam_player_01 (Variables|Default|GetShotgunMagAmmo))
  (Variables|/Game/Lucas/BP_Unreal_Jam_Player_01.BP_Unreal_Jam_Player_01_C|SetShotgunTotalAmmo _asbp_unreal_jam_player_01 (Variables|Default|GetShotgunTotalAmmo))
  (Variables|/Game/Lucas/BP_Unreal_Jam_Player_01.BP_Unreal_Jam_Player_01_C|SetOwnedWeapons _asbp_unreal_jam_player_01 (Variables|Default|GetOwnedWeapons))
  (Default|SwitchWeapon _asbp_unreal_jam_player_01 (Variables|Default|GetCurrentWeapon))
  (Variables|/Game/Lucas/BP_Unreal_Jam_Health_System_01.BP_Unreal_Jam_Health_System_01_C|SetHealth (Variables|/Game/Lucas/BP_Unreal_Jam_Player_01.BP_Unreal_Jam_Player_01_C|GetBP_Unreal_Jam_Health_System_01 _asbp_unreal_jam_player_01) (Variables|Default|GetHealth))
  (Variables|/Game/Lucas/BP_Unreal_Jam_Health_System_01.BP_Unreal_Jam_Health_System_01_C|SetRemainRestoreHealth (Variables|/Game/Lucas/BP_Unreal_Jam_Player_01.BP_Unreal_Jam_Player_01_C|GetBP_Unreal_Jam_Health_System_01 _asbp_unreal_jam_player_01) (Variables|Default|GetRemainHelth)))

(fn PlayTakeSound
  (bind _array (Utilities|Array|MakeArray "/Game/Dialogues/Gameplay/A_01_That_What_I_Need_01.A_01_That_What_I_Need_01" "/Game/Dialogues/Gameplay/A_01_That_What_I_Need_02.A_01_That_What_I_Need_02" "/Game/Dialogues/Gameplay/A_01_That_What_I_Need_03.A_01_That_What_I_Need_03"))
  (if (Math|Random|RandomBoolwithWeight 0.25)
    (Audio|PlaySound2D (Utilities|Array|Get(acopy) _array (Math|Random|RandomIntegerinRange 0 (Utilities|Array|LastIndex _array))) 1.0 1.0 0.0 0 0)))

(fn PlayKillSound
  (bind _array (Utilities|Array|MakeArray "/Game/Dialogues/Gameplay/A_02_In_Your_Face_01.A_02_In_Your_Face_01" "/Game/Dialogues/Gameplay/A_02_In_Your_Face_02.A_02_In_Your_Face_02" "/Game/Dialogues/Gameplay/A_02_In_Your_Face_03.A_02_In_Your_Face_03" "/Game/Dialogues/Gameplay/A_02_In_Your_Face_04.A_02_In_Your_Face_04"))
  (if (Math|Random|RandomBoolwithWeight 0.25)
    (Audio|PlaySound2D (Utilities|Array|Get(acopy) _array (Math|Random|RandomIntegerinRange 0 (Utilities|Array|LastIndex _array))) 1.0 1.0 0.0 0 0)))

(fn PlayHurtSound
  (bind _array (Utilities|Array|MakeArray "/Game/Dialogues/Gameplay/A_03_It_Hurts_01.A_03_It_Hurts_01" "/Game/Dialogues/Gameplay/A_03_It_Hurts_02.A_03_It_Hurts_02"))
  (bind _array_2 (Utilities|Array|MakeArray "/Game/Dialogues/Gameplay/A_04_Pain_Scream_01.A_04_Pain_Scream_01" "/Game/Dialogues/Gameplay/A_04_Pain_Scream_02.A_04_Pain_Scream_02" "/Game/Dialogues/Gameplay/A_04_Pain_Scream_03.A_04_Pain_Scream_03" "/Game/Dialogues/Gameplay/A_04_Pain_Scream_04.A_04_Pain_Scream_04"))
  (if (Math|Random|RandomBoolwithWeight 0.25)
    (Audio|PlaySound2D (Utilities|Array|Get(acopy) _array (Math|Random|RandomIntegerinRange 0 (Utilities|Array|LastIndex _array))) 1.0 1.0 0.0 0 0)
    (else
      (Audio|PlaySound2D (Utilities|Array|Get(acopy) _array_2 (Math|Random|RandomIntegerinRange 0 (Utilities|Array|LastIndex _array_2))) 1.0 1.0 0.0 0 0))))