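; Player health component that tracks damage, healing and death, disabling its tick and broadcasting OnPlayerDead when health runs out.
; Each tick runs passive regeneration up to a cap after a post-damage delay, alongside gradual restoration from a pooled aid amount.
; Using aid adds to that pool and skips the regen delay.
; Missing health drives a screen-blood parameter in a Material Parameter Collection through a curve.
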(event EventBeginPlay)

(event EventTick
  (params (DeltaSeconds :type Float%20%28single-precision%29))
  (CallFunction|RegenHealth DeltaSeconds)
  (CallFunction|RestoreHealth DeltaSeconds)
  (CallFunction|UpdateScreenBlood DeltaSeconds))

(fn UpdateScreenBlood
  (params (DeltaTime :type Float%20%28single-precision%29))
  (Rendering|Material|SetScalarParameterValue "/Game/Lucas/Mat/MPC_Unreal_Jam_Collection_01.MPC_Unreal_Jam_Collection_01" "ScreenRed" (Math|Curves|GetFloatValue (Variables|Default|GetScreenBloodCurve) (- 1.0 (/ (Variables|Default|GetHealth) 1e+02))) :!class /Script/Engine.KismetMaterialLibrary))

(fn RegenHealth
  (params (DeltaTime :type Float%20%28single-precision%29))
  (if (>= (Variables|Default|GetCurrentRegenDelay) (Variables|Settings|GetRegenDelay))
    (if (< (Variables|Default|GetHealth) (Variables|Settings|GetMaxRegenHealth))
      (Variables|Default|SetHealth (Math|Float|Clamp(Float) (+ (Variables|Default|GetHealth) (* DeltaTime (Variables|Settings|GetRegenPerSecond))) 0.0 (Variables|Settings|GetMaxRegenHealth))))
    (else
      (Variables|Default|SetCurrentRegenDelay (+ DeltaTime (Variables|Default|GetCurrentRegenDelay))))))

(fn RestoreHealth
  (params (DeltaTime :type Float%20%28single-precision%29))
  (if (and (< (Variables|Default|GetHealth) 1e+02) (> (Variables|Default|GetRemainRestoreHealth) 0.0))
    (LocalVariables|SetCurrentHealthToRestore (Math|Float|Clamp(Float) (* DeltaTime (Variables|Settings|GetRestorePerSecond)) 0.0 (Variables|Default|GetRemainRestoreHealth)))
    (LocalVariables|SetCurrentMaxRestoreHealth (Math|Float|Clamp(Float) (+ (Variables|Default|GetHealth) (Variables|Default|GetRemainRestoreHealth)) 0.0 1e+02))
    (Variables|Default|SetHealth (Math|Float|Clamp(Float) (+ (Variables|Default|GetHealth) (LocalVariables|GetCurrentHealthToRestore)) 0.0 1e+02))
    (Variables|Default|SetRemainRestoreHealth (Math|Float|Clamp(Float) (- (Variables|Default|GetRemainRestoreHealth) (LocalVariables|GetCurrentHealthToRestore)) 0.0 (Variables|Default|GetRemainRestoreHealth)))
    (if (>= (Variables|Default|GetHealth) 1e+02)
      (Variables|Default|SetRemainRestoreHealth 0.0))))

(fn CanUseAid
  (return (< (+ (Variables|Default|GetHealth) (Variables|Default|GetRemainRestoreHealth)) 1e+02)))

(fn AddRestoreHealth
  (params (RestoreHealth :type Float%20%28single-precision%29))
  (Variables|Default|SetRemainRestoreHealth (+ RestoreHealth (Variables|Default|GetRemainRestoreHealth)))
  (Variables|Default|SetCurrentRegenDelay (Variables|Settings|GetRegenDelay)))

(fn ReceiveDamage
  (params (Damage :type Float%20%28single-precision%29))
  (Variables|Default|SetHealth (Math|Float|Clamp(Float) (- (Variables|Default|GetHealth) Damage) 0.0 1e+02))
  (if (<= (Variables|Default|GetHealth) 0.1)
    (Components|Tick|SetComponentTickEnabled false)
    (Default|CallOnPlayerDead)
    (else
      (Variables|Default|SetCurrentRegenDelay 0.0))))