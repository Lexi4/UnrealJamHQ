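; Player controller for an Unreal Jam game that handles interaction, weapon switching, reload, flashlight and screen fades for the player pawn.
; Each tick, a short trace along the player's look finds interface-implementing actors, showing their prompt through the game instance only when the text changes.
; The Action input triggers the focused actor if it allows interaction.
; FadeIn and FadeOut drive a material parameter collection's ScreenFade with one timeline played forward or reversed.
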(event Custom|FadeIn
  (bind _newtrack_0 (Timeline|Timeline_0 PlayFromStart)
    (:Update
      (Rendering|Material|SetScalarParameterValue "/Game/Lucas/Mat/MPC_Unreal_Jam_Collection_01.MPC_Unreal_Jam_Collection_01" "ScreenFade" _newtrack_0 :!class /Script/Engine.KismetMaterialLibrary))))

(event Custom|FadeOut
  (bind _newtrack_0 (Timeline|Timeline_0 ReverseFromEnd)
    (:Update
      (Rendering|Material|SetScalarParameterValue "/Game/Lucas/Mat/MPC_Unreal_Jam_Collection_01.MPC_Unreal_Jam_Collection_01" "ScreenFade" _newtrack_0 :!class /Script/Engine.KismetMaterialLibrary))))

(event EventBeginPlay)

(event EventTick
  (params (DeltaSeconds :type Float%20%28single-precision%29))
  (bind _player (CallFunction|GetUJPlayer))
  (bind (_position _direction) (Default|GetLook _player))
  (Utilities|IsValid (CallFunction|GetUJPlayer)
    (:Is%20Valid
      (bind (_outhit _returnvalue) (Collision|LineTraceByChannel _position (+ _position (* _direction 3e+02)) "TraceTypeQuery3" true (Utilities|Array|MakeArray (CallFunction|GetUJPlayer)) "None"))
      (if _returnvalue
        (CallFunction|NewInteractionActor (.HitActor (Collision|BreakHitResult _outhit)))
        (else
          (CallFunction|NewInteractionActor))))))

(event Input|ActionEvents|InputActionAction
  (params (Key :type Key%20Structure))
  (:Pressed
    (Utilities|IsValid (Variables|Default|GetCurrentInteractionActor)
      (:Is%20Valid
        (if (Utilities|DoesObjectImplementInterface (Variables|Default|GetCurrentInteractionActor) "/Game/Lucas/BP_Unreal_Jam_Interaction_Interface_01.BP_Unreal_Jam_Interaction_Interface_01_C")
          (bind _bcaninteract (Class|BPUnrealJamInteractionInterface01|CanInteract(Message) (Variables|Default|GetCurrentInteractionActor)))
          (if _bcaninteract
            (Class|BPUnrealJamInteractionInterface01|MakeAction(Message) (Variables|Default|GetCurrentInteractionActor))))))))

(event Input|ActionEvents|InputActionFirstWeapon
  (params (Key :type Key%20Structure))
  (:Pressed
    (Default|SwitchWeapon (CallFunction|GetUJPlayer) "NewEnumerator0")))

(event Input|ActionEvents|InputActionSecondWeapon
  (params (Key :type Key%20Structure))
  (:Pressed
    (Default|SwitchWeapon (CallFunction|GetUJPlayer) "NewEnumerator1")))

(event Input|ActionEvents|InputActionReload
  (params (Key :type Key%20Structure))
  (:Pressed
    (Default|Reload (CallFunction|GetUJPlayer))))

(event Input|ActionEvents|InputActionThirdWeapon
  (params (Key :type Key%20Structure))
  (:Pressed
    (Default|SwitchWeapon (CallFunction|GetUJPlayer) "NewEnumerator2")))

(event Input|ActionEvents|InputActionFlashlight
  (params (Key :type Key%20Structure))
  (bind _player (CallFunction|GetUJPlayer))
  (bind _spotlight (Variables|/Game/Lucas/BP_Unreal_Jam_Player_01.BP_Unreal_Jam_Player_01_C|GetSpotLight _player))
  (:Pressed
    (Utilities|FlowControl|FlipFlop
      (:A
        (Rendering|Components|Light|SetIntensity _spotlight 7.5e+03))
      (:B
        (Rendering|Components|Light|SetIntensity _spotlight 0.0)))))

(fn ConstructionScript)

(fn GetUJPlayer
  (bind _asbp_unreal_jam_player_01 (Utilities|Casting|CastToBP_Unreal_Jam_Player_01 (Pawn|GetControlledPawn))
    (:then
      (return _asbp_unreal_jam_player_01))
    (:CastFailed
      (return 0))))

(fn NewInteractionActor
  (params (NewInteractionActor :type Actor%20Object%20Reference))
  (Variables|Default|SetCurrentInteractionActor NewInteractionActor)
  (Utilities|IsValid (Variables|Default|GetCurrentInteractionActor)
    (:Is%20Valid
      (if (Utilities|DoesObjectImplementInterface (Variables|Default|GetCurrentInteractionActor) "/Game/Lucas/BP_Unreal_Jam_Interaction_Interface_01.BP_Unreal_Jam_Interaction_Interface_01_C")
        (bind _bcaninteract (Class|BPUnrealJamInteractionInterface01|CanInteract(Message) (Variables|Default|GetCurrentInteractionActor)))
        (if _bcaninteract
          (bind _actiontext (Class|BPUnrealJamInteractionInterface01|GetActionText(Message) (Variables|Default|GetCurrentInteractionActor)))
          (bind _output_get (LocalVariables|SetCurrentText _actiontext))
          (if (not (Utilities|Enum|Equal(Enum) _output_get (Variables|Default|GetLastActionText)))
            (bind _output_get_2 (Variables|Default|SetLastActionText (LocalVariables|GetCurrentText)))
            (Default|EnabledActionStroke (CallFunction|GetUJGameInstance) _output_get_2))
          (else
            (Variables|Default|SetLastActionText "" :!label _label)
            (Default|DisableActionStroke (CallFunction|GetUJGameInstance))))
        (else
          (goto _label))))
    (:Is%20Not%20Valid
      (goto _label))))